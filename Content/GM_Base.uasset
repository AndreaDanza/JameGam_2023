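; GM_Base, apparently the base game mode, tracks the level's enemy count and signals basement door destruction.
; BeginPlay counts actors tagged "Enemye", stores that as the total and remaining counts, and debug-prints both.
; AnEnemyDie decrements the remaining count and calls DestroyBaismentDoor on every death, with no zero check in this graph.
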(event Custom|AnEnemyDie
  (Variables|Default|SetEnemyeLeft (- (Variables|Default|GetEnemyeLeft) 1))
  (Default|CallDestroyBaismentDoor))

(event EventBeginPlay
  (bind _outactors (Actor|GetAllActorswithTag "Enemye"))
  (bind _output_get (Variables|Default|SetEnemyeTotal (Utilities|Array|Length _outactors)))
  (Development|PrintString (Utilities|String|ToString(Integer) _output_get) true true "(R=1.000000,G=0.000000,B=0.005552,A=1.000000)")
  (bind _output_get_2 (Variables|Default|SetEnemyeLeft _output_get))
  (Development|PrintString (Utilities|String|ToString(Integer) _output_get_2)))

(event EventTick
  (params (DeltaSeconds :type Float%20%28single-precision%29)))

(fn ConstructionScript)