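; BP_DogTrue is an enemy Blueprint that drives a Princess boss battle health bar through GM_Base.
; Each Tick it binds widget creation to the game mode's DestroyLockerDoor event and broadcasts its Life against a fixed maximum via GetPrincessHealth.
; When DestroyLockerDoor fires, it creates the PrincessBossBattle widget and adds it to the viewport.
; On Destroyed, it collapses that health bar.
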(event Custom|CreateHealth
  (params (Test :type Text))
  (bind _returnvalue (UserInterface|CreateWidget "/Game/Widget/PrincessBossBattle.PrincessBossBattle_C"))
  (bind _output_get (Variables|Default|SetHealthBar _returnvalue))
  (UserInterface|Viewport|AddtoViewport _returnvalue 0))

(event EventBeginPlay)

(event Collision|EventActorBeginOverlap
  (params (OtherActor :type Actor%20Object%20Reference)))

(event EventTick
  (params (DeltaSeconds :type Float%20%28single-precision%29))
  (|CallParentFunction DeltaSeconds)
  (bind _asgm_base (Utilities|Casting|CastToGM_Base (Game|GetGameMode)))
  (EventDispatchers|BindEventtoDestroyLockerDoor _asgm_base (delegate Custom|CreateHealth))
  (Default|CallGetPrincessHealth _asgm_base 5e+01 (Math|Conversions|ToFloat(Integer) (Variables|Default|GetLife))))

(event EventDestroyed
  (Widget|SetVisibility (Variables|Default|GetHealthBar) "Collapsed"))

(fn ConstructionScript
  (|CallParentFunction))