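; Black dog enemy character that chases the player on sight through PawnSensing and AI MoveTo.
; Range overlap opens a gate that lets Tick damage the player after an AttackSpeed delay, switching run and attack flipbooks.
; Hammer overlaps during the player's Hummerata state subtract Life, knocking the dog back with a DoOnce cooldown or destroying it and notifying GM_Base.
; Life displays as text, and construction scales both trigger volumes.
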(event OnComponentBeginOverlap(Range)
  (params (OverlappedComponent :type Primitive%20Component%20Object%20Reference) (OtherActor :type Actor%20Object%20Reference) (OtherComp :type Primitive%20Component%20Object%20Reference) (OtherBodyIndex :type Integer) (bFromSweep :type Boolean) (SweepResult :type Hit%20Result%20Structure%20%28by%20ref%29))
  (Utilities|FlowControl|Gate true) ; enters at Open
)

(event OnSeePawn(PawnSensing)
  (params (Pawn :type Pawn%20Object%20Reference))
  (Variables|Default|SetisSeePlayer true)
  (CallFunction|ISee))

(event OnComponentEndOverlap(Range)
  (params (OverlappedComponent :type Primitive%20Component%20Object%20Reference) (OtherActor :type Actor%20Object%20Reference) (OtherComp :type Primitive%20Component%20Object%20Reference) (OtherBodyIndex :type Integer))
  (Sprite|SetFlipbook (Variables|Default|GetSprite) (Variables|Default|GetRunn))
  (Utilities|FlowControl|Gate true) ; enters at Close
)

(event OnComponentBeginOverlap(Damage)
  (params (OverlappedComponent :type Primitive%20Component%20Object%20Reference) (OtherActor :type Actor%20Object%20Reference) (OtherComp :type Primitive%20Component%20Object%20Reference) (OtherBodyIndex :type Integer) (bFromSweep :type Boolean) (SweepResult :type Hit%20Result%20Structure%20%28by%20ref%29))
  (bind _returnvalue (Transformation|GetActorLocation OtherActor))
  (bind _capsulecomponent (Variables|Default|GetCapsuleComponent))
  (bind _returnvalue_2 (Transformation|GetWorldLocation _capsulecomponent))
  (bind _returnvalue_3 (Math|Vector|GetUnitDirection(Vector) _returnvalue _returnvalue_2))
  (bind _returnvalue_4 (Math|Vector|MakeVector (.x _returnvalue_3) (.y _returnvalue_3) 0.0))
  (bind _returnvalue_5 (Math|Vector|Normalize _returnvalue_4))
  (bind _returnvalue_6 (Math|Vector|MakeVector (.x _returnvalue_5) (.y _returnvalue_5) 0.0))
  (bind _returnvalue_7 (* _returnvalue_6 2e+02))
  ;[1 1 1] TakeDamage
  (if (not (== OtherComp (Actor|GetComponentbyClass OtherActor "/Script/Engine.SphereComponent")))
    (bind _ashammer (Utilities|Casting|CastToHammer OtherActor))
    (bind _asbp_top_down_char (Utilities|Casting|CastToBP_TopDown_Char (Game|GetPlayerCharacter 0)))
    (if (Variables|/Game/Character/BP_TopDown_Char.BP_TopDown_Char_C|GetHummerata _asbp_top_down_char)
      (Utilities|FlowControl|DoOnce false :!label _label
        (:Completed
          (bind _output_get (Variables|Default|SetLife (- (Variables|Default|GetLife) (Variables|/Game/Character/Hammer/Hammer.Hammer_C|GetHammerDMG _ashammer))))
          (if (<= _output_get 0)
            (Actor|DestroyActor)
            (bind _asgm_base (Utilities|Casting|CastToGM_Base (Game|GetGameMode)))
            (Default|AnEnemyDie _asgm_base)
            (else
              (Character|LaunchCharacter (Math|Vector|MakeVector (.x _returnvalue_7) (.y _returnvalue_7) 0.0) false false)
              (Utilities|FlowControl|Delay 0.7)
              (goto _label Reset))))))))

(event Custom|iSee
  (if (Variables|Default|GetisSeePlayer)
    (bind _asbp_top_down_char (Utilities|Casting|CastToBP_TopDown_Char (stale OnSeePawn(PawnSensing) Pawn)))
    (AI|AIMoveTo self "0, 0, 0" _asbp_top_down_char 5.0 false)))

(event EventBeginPlay
  (Sprite|SetFlipbook (Variables|Default|GetSprite) (Variables|Default|GetRunn))
  (Variables|/Script/Engine.CharacterMovementComponent|SetMaxAcceleration (Variables|Character|GetCharacterMovement) (/ (Variables|Default|GetSpeed) (.z (Transformation|GetWorldScale (Variables|Default|GetSprite))))))

(event EventTick
  (params (DeltaSeconds :type Float%20%28single-precision%29))
  (Rendering|Components|TextRender|SetText (Variables|Default|GetTextRender) (Utilities|Text|ToText(Integer) (Variables|Default|GetLife)))
  (if (== (stale OnComponentBeginOverlap(Range) OtherActor) (Game|GetPlayerCharacter 0))
    (bind _asbp_top_down_char (Utilities|Casting|CastToBP_TopDown_Char (stale OnComponentBeginOverlap(Range) OtherActor)))
    (Utilities|FlowControl|Delay (Variables|Default|GetAttackSpeed))
    (Utilities|FlowControl|Gate true
      (:Exit
        (Default|TakeDamege _asbp_top_down_char self)
        (Sprite|SetFlipbook (Variables|Default|GetSprite) (Variables|Default|GetAttack))))))

(fn ConstructionScript
  (Transformation|SetRelativeScale3D (Variables|Default|GetDamage) (Variables|Default|GetTakeDMG))
  (Transformation|SetRelativeScale3D (Variables|Default|GetRange) (Variables|Default|GetRangeScale)))